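; Learning Agents interactor that defines observations for agents following a track, with no actions implemented.
; Setup creates planar track position and direction, angle and car velocity observations, plus a spline helper using the BP_PatrolSpline spline.
; Per-agent updates write only a goal position relative to each agent's transform, but that observation's creation is unconnected, and the track and velocity observations are never set.
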(event EventSetObservations
  (params (AgentIds :type Array%20of%20Integers))
  (for _array_element AgentIds
    (Class|PositionObservation|SetPositionObservation (Variables|Default|GetGoalLocationObservation) _array_element (Variables|Default|GetGoalLocation) (.location (Transformation|GetActorTransform (Class|LearningAgentsManagerComponent|GetAgent _array_element "/Game/Blueprints/Characters/BP_LearningAgent.BP_LearningAgent_C"))) (.rotation (Transformation|GetActorTransform (Class|LearningAgentsManagerComponent|GetAgent _array_element "/Game/Blueprints/Characters/BP_LearningAgent.BP_LearningAgent_C"))))))

(event EventSetupActions)

(event EventGetActions
  (params (AgentIds :type Array%20of%20Integers)))

(event EventSetupObservations
  (Utilities|FlowControl|Sequence
    (:then_0
      (bind _returnvalue (Class|PlanarPositionObservation|AddPlanarPositionObservation 0 "TrackPositionObservation" 1e+02 "1.000000,0.000000,0.000000" "0.000000,1.000000,0.000000"))
      (Variables|Default|SetTrackPositionObservation _returnvalue)
      (bind _returnvalue_2 (Class|PlanarDirectionObservation|AddPlanarDirectionObservation 0 "TrackDirectionObservation" 1.0 "1.000000,0.000000,0.000000" "0.000000,1.000000,0.000000"))
      (Variables|Default|SetTrackDirectionObservation _returnvalue_2))
    (:then_1
      (bind _returnvalue_3 (Class|AngleObservation|AddAngleObservation 0 "TrackGlobalPositionObservation" 1.0))
      (Variables|Default|SetTrackGlobalPositionObservation _returnvalue_3)
      (bind _returnvalue_4 (Class|PlanarVelocityObservation|AddPlanarVelocityObservation 0 "CarVelocityObservation" 2e+02 "1.000000,0.000000,0.000000" "0.000000,1.000000,0.000000"))
      (Variables|Default|SetCarVelocityObservation _returnvalue_4))
    (:then_2
      (bind _returnvalue_5 (Class|SplineComponentHelper|AddSplineComponentHelper 0 "SplineComponentHelper"))
      (Variables|Default|SetSplineComponentHelper _returnvalue_5)
      (bind _returnvalue_6 (Actor|GetActorOfClass "/Game/Blueprints/Learning/BP_PatrolSpline.BP_PatrolSpline_C"))
      (Variables|Default|SetTrackSpline (Variables|/Game/Blueprints/Learning/BP_PatrolSpline.BP_PatrolSpline_C|GetSpline _returnvalue_6)))))